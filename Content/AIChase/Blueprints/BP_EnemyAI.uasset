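; Enemy AI character that chases the player once pawn sensing spots them, then attacks on reaching them.
; A successful AI move applies damage and launches the player along their own up and forward vectors.
; A self-repeating RunAway event moves away from the player at constant height, but nothing outside it calls it; the R key only sets a flag.
; Montage attack and debug print logic are disconnected.
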(event `self.PawnSensing.OnSeePawn`
  (params (Pawn :type "Pawn Object Reference"))
  (set `self.isSeeingPlayer?` true)
  (`self.FollowPlayer`))

(event `FollowPlayer`
  (bind _returnvalue (`GameplayStatics.GetPlayerCharacter` 0))
  (set `self.canAttack?` true)
  (if (`self.isSeeingPlayer?`)
    (`|AIMoveTo` self (0.0 0.0 0.0) (`GameplayStatics.GetPlayerCharacter` 0) 70.0
      (:`OnSuccess`
        (set `self.isCatched?` true)
        (if (`self.isCatched?`)
          (set `self.isCatched?` false)
          (bind _asbp_first_person_character (cast `/Game/FirstPerson/Blueprints/BP_FirstPersonCharacter` (`GameplayStatics.GetPlayerCharacter` 0)))
          ;[1 0.02122 0] Damage
          (`GameplayStatics.ApplyDamage` _asbp_first_person_character 10.0 null self)
          ;[1 0.3645 0.3744] Adding Impulse to Upward
          (`CharacterMovementComponent.AddImpulse` (`Character.CharacterMovement` _asbp_first_person_character) (* (`self.GetActorUpVector` _returnvalue) 500.0) true)
          ;[0.2891 0.5373 1] Adding Impulse to Forward
          (`CharacterMovementComponent.AddImpulse` (`Character.CharacterMovement` _asbp_first_person_character) (* (`self.GetActorForwardVector` _returnvalue) 1500.0) true))))))

(event `self.ReceiveBeginPlay`
  (bind _asbp_first_person_character (cast `/Game/FirstPerson/Blueprints/BP_FirstPersonCharacter` (`GameplayStatics.GetPlayerCharacter` 0)))
  (set `self.Character REF` _asbp_first_person_character))

(event `Key|R`
  (params (Key :type "Key Structure"))
  (:`Pressed`
    (set `self.RunAway?` true)))

(event `RunAway`
  (bind _returnvalue (`self.K2_GetActorLocation`))
  (`|AIMoveTo` self (`KismetMathLibrary.MakeVector` (.x (+ _returnvalue (* (`KismetMathLibrary.GetForwardVector` (`KismetMathLibrary.FindLookAtRotation` _returnvalue (`self.K2_GetActorLocation` (`self.Character REF`)))) -500.0))) (.y (+ _returnvalue (* (`KismetMathLibrary.GetForwardVector` (`KismetMathLibrary.FindLookAtRotation` _returnvalue (`self.K2_GetActorLocation` (`self.Character REF`)))) -500.0))) (.z _returnvalue)) null
    (:`OnSuccess`
      _)
    (:`OnFail`
      _))
  (`self.RunAway`))

(fn `UserConstructionScript`)