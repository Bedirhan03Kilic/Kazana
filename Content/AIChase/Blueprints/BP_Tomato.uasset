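; BP_Tomato is an actor that damages the first-person player character on a hit, then destroys itself and plays the Goose sound.
; The Hit event casts to BP_FirstPersonCharacter, applies damage and passes its CharacterMovement to two helper functions.
; One lowers walk speed and jump velocity, the other sets fixed higher values immediately afterwards with no delay, so the slowdown does not persist.
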(event `self.ReceiveHit`
  (params (MyComp :type "PrimitiveComponent Object Reference") (Other :type "Actor Object Reference") (OtherComp :type "PrimitiveComponent Object Reference") (bSelfMoved :type Boolean) (HitLocation :type "Vector Structure") (HitNormal :type "Vector Structure") (NormalImpulse :type "Vector Structure") (Hit :type "HitResult Structure (by ref)"))
  (bind _asbp_first_person_character (cast `/Game/FirstPerson/Blueprints/BP_FirstPersonCharacter` Other))
  (`GameplayStatics.ApplyDamage` _asbp_first_person_character 10.0)
  (`self.K2_DestroyActor`)
  (`self.Decrease Speed and Height of Jump` (`Character.CharacterMovement` _asbp_first_person_character) (`Character.CharacterMovement` _asbp_first_person_character))
  (`self.Returning Speed And Jump Values Back` (`Character.CharacterMovement` _asbp_first_person_character) (`Character.CharacterMovement` _asbp_first_person_character))
  (`GameplayStatics.PlaySound2D` "/Game/Sounds/Goose.Goose" 1.0 1.0 0.0 null null))

(fn `Decrease Speed and Height of Jump`
  (params (self2 :type "CharacterMovementComponent Object Reference") (self3 :type "CharacterMovementComponent Object Reference"))
  (set `CharacterMovementComponent.MaxWalkSpeed` 100.0 self2)
  (set `CharacterMovementComponent.JumpZVelocity` 100.0 self3))

(fn `Returning Speed And Jump Values Back`
  (params (self2 :type "CharacterMovementComponent Object Reference") (self3 :type "CharacterMovementComponent Object Reference"))
  (set `CharacterMovementComponent.JumpZVelocity` 420.0 self2)
  (set `CharacterMovementComponent.MaxWalkSpeed` 600.0 self3))

(fn `UserConstructionScript`)