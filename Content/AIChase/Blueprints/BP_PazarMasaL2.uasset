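; BP_PazarMasaL2 is a one-time interactable that spawns a Bp_Chick3 AI pawn when the player presses E nearby.
; Its Box overlap shows a Widget and enables input while BP_FirstPersonCharacter is inside, reversing both on exit.
; E passes a DoOnce, spawns the pawn at an offset from the actor, launches it with a delayed velocity impulse, then hides the prompt and disables input.
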(event `self.Box.OnComponentBeginOverlap`
  (params (OverlappedComponent :type "PrimitiveComponent Object Reference") (OtherActor :type "Actor Object Reference") (OtherComp :type "PrimitiveComponent Object Reference") (OtherBodyIndex :type Integer) (bFromSweep :type Boolean) (SweepResult :type "HitResult Structure (by ref)"))
  (cast `/Game/FirstPerson/Blueprints/BP_FirstPersonCharacter` OtherActor)
  (`SceneComponent.SetVisibility` (`self.Widget`) true false)
  (`self.EnableInput` (`GameplayStatics.GetPlayerController` 0)))

(event `self.Box.OnComponentEndOverlap`
  (params (OverlappedComponent :type "PrimitiveComponent Object Reference") (OtherActor :type "Actor Object Reference") (OtherComp :type "PrimitiveComponent Object Reference") (OtherBodyIndex :type Integer))
  (cast `/Game/FirstPerson/Blueprints/BP_FirstPersonCharacter` OtherActor)
  (`SceneComponent.SetVisibility` (`self.Widget`) false false)
  (`self.DisableInput` (`GameplayStatics.GetPlayerController` 0)))

(event `Key|E`
  (params (Key :type "Key Structure"))
  (:`Pressed`
    (`/Engine/EditorBlueprintResources/StandardMacros.DoOnce` false
      (:`Completed`
        (bind _returnvalue (`AIBlueprintHelperLibrary.SpawnAIFromClass` "/Game/AIChase/Blueprints/Bp_Chick3.Bp_Chick3_C" null (+ (`self.K2_GetActorLocation`) (100.0 0.0 100.0)) (struct) true null))
        (bind _asbp_chick_3 (cast `/Game/AIChase/Blueprints/Bp_Chick3` _returnvalue))
        (`KismetSystemLibrary.Delay` 0.2)
        (`CharacterMovementComponent.AddImpulse` (`Character.CharacterMovement` _asbp_chick_3) (100.0 0.0 500.0) true)
        (`SceneComponent.SetVisibility` (`self.Widget`) false false)
        (`self.DisableInput` null)))))

(fn `UserConstructionScript`)