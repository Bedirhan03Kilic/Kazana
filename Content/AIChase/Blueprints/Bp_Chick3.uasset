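; Chick AI that moves to a new spot each time it senses the player, apparently by hearing.
; Successful perception updates advance a counter that sends it through three locations and then a last one.
; The fourth move increments the player's ChickAmount as soon as it is issued, without waiting for arrival.
; Tick re-fetches the player reference every frame; the sight handler is empty and the follow logic is never triggered.
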(event `self.ReceiveBeginPlay`
  (set `self.Relocate` 0))

(event `self.PawnSensing.OnSeePawn`
  (params (Pawn :type "Pawn Object Reference"))
  ;[1 1 1] Chick Follow Player On See
)

(event `Random Roam`
  ;[1 1 1] AI HEAR
  ;;[1 1 1] Chick Follow Player On See
  (`|AIMoveTo` self (-360.0 1430.0 1550.0) (`GameplayStatics.GetPlayerCharacter` 0)
    (:`OnSuccess`
      (set `self.canfollow?` false)
      (`KismetSystemLibrary.Delay` 2.0)
      (set `self.canfollow?` true))))

(event `self.AIPerception.OnTargetPerceptionUpdated`
  (params (Actor :type "Actor Object Reference") (Stimulus :type "AIStimulus Structure"))
  (bind _bpref2 (`self.bpREF2`))
  ;[1 1 1] AI HEAR
  (cast `/Game/FirstPerson/Blueprints/BP_FirstPersonCharacter` Actor)
  (if (`.bSuccessfullySensed` (break `AIStimulus` Stimulus))
    (set `self.Relocate` (+ (`self.Relocate`) 1))
    (switch `int` (`self.Relocate`)
      (:`1`
        (`|AIMoveTo` self (`self.Location1`) null))
      (:`2`
        (`|AIMoveTo` self (`self.Location2`) null))
      (:`3`
        (`|AIMoveTo` self (`self.Location3`) null))
      (:`4`
        (`|AIMoveTo` self (`self.LastLocation`) null
          (:`then`
            (set `/Game/FirstPerson/Blueprints/BP_FirstPersonCharacter.ChickAmount` (+ (`/Game/FirstPerson/Blueprints/BP_FirstPersonCharacter.ChickAmount` _bpref2) 1) _bpref2)))))))

(event `self.ReceiveTick`
  (params (DeltaSeconds :type "Float (single-precision)"))
  (bind _outactors (`GameplayStatics.GetAllActorsOfClass` "/Game/FirstPerson/Blueprints/BP_FirstPersonCharacter.BP_FirstPersonCharacter_C"))
  (set `self.bpREF2` (`|GetArrayItem` _outactors)))

(fn `UserConstructionScript`)