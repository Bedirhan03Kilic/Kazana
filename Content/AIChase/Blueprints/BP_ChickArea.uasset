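; BP_ChickArea is a trigger area where the player presses E to send a chick to a fixed world location.
; Box overlap shows a prompt widget and enables input, and leaving reverses both.
; E sets CanChicksGo, issues AIMoveTo on the chick reference, then hides the widget and disables input without waiting for arrival.
; Tick refreshes that reference every frame with the first Bp_Chick found in the level.
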(event `self.Box.OnComponentBeginOverlap`
  (params (OverlappedComponent :type "PrimitiveComponent Object Reference") (OtherActor :type "Actor Object Reference") (OtherComp :type "PrimitiveComponent Object Reference") (OtherBodyIndex :type Integer) (bFromSweep :type Boolean) (SweepResult :type "HitResult Structure (by ref)"))
  (`SceneComponent.SetVisibility` (`self.Widget`) true false)
  (`self.EnableInput` (`GameplayStatics.GetPlayerController` 0)))

(event `self.Box.OnComponentEndOverlap`
  (params (OverlappedComponent :type "PrimitiveComponent Object Reference") (OtherActor :type "Actor Object Reference") (OtherComp :type "PrimitiveComponent Object Reference") (OtherBodyIndex :type Integer))
  (`SceneComponent.SetVisibility` (`self.Widget`) false false)
  (`self.DisableInput` (`GameplayStatics.GetPlayerController` 0)))

(event `Key|E`
  (params (Key :type "Key Structure"))
  (:`Pressed`
    (set `self.CanChicksGo?` true)
    (`|AIMoveTo` (`self.ChickRefferance`) (-482.469287 19421.738637 3695.847477) null
      (:`then`
        (`SceneComponent.SetVisibility` (`self.Widget`) false false)
        (`self.DisableInput` null)))))

(event `self.ReceiveTick`
  (params (DeltaSeconds :type "Float (single-precision)"))
  (bind _outactors (`GameplayStatics.GetAllActorsOfClass` "/Game/AIChase/Blueprints/Bp_Chick.Bp_Chick_C"))
  (set `self.ChickRefferance` (`|GetArrayItem` _outactors)))

(fn `UserConstructionScript`)