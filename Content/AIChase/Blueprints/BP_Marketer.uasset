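; BP_Marketer is an AI enemy that throws tomatoes at the first-person player on sight.
; PawnSensing turns it toward the player, then a delayed Throw animation precedes spawning a BP_Tomato launched along the spawn point's forward vector.
; A CanAttack flag and delay enforce a cooldown between throws.
; Two helper functions, not called here, reduce and restore walk speed and jump height on the movement components passed in.
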(event `self.PawnSensing.OnSeePawn`
  (params (Pawn :type "Pawn Object Reference"))
  (bind _asbp_first_person_character (cast `/Game/FirstPerson/Blueprints/BP_FirstPersonCharacter` Pawn))
  (`self.K2_SetActorRotation` (`KismetMathLibrary.FindRelativeLookAtRotation` (`KismetMathLibrary.Conv_VectorToTransform` (`self.K2_GetActorLocation`)) (`self.K2_GetActorLocation` _asbp_first_person_character)))
  (if (`self.CanAttack?`)
    (`KismetSystemLibrary.Delay` 1.0)
    (`SkeletalMeshComponent.PlayAnimation` (`self.Mesh`) "/Game/AIChase/AI_Animation/Throw.Throw" false)
    (`KismetSystemLibrary.Delay` 1.0)
    (bind _returnvalue (`|SpawnActorFromClass` "/Game/AIChase/Blueprints/BP_Tomato.BP_Tomato_C" (`SceneComponent.K2_GetComponentToWorld` (`self.SpawnProjectileLocation`)) "Undefined" "MultiplyWithRoot" null null))
    (`PrimitiveComponent.SetPhysicsLinearVelocity` (`/Game/AIChase/Blueprints/BP_Tomato.Sphere` _returnvalue) (* (`SceneComponent.GetForwardVector` (`self.SpawnProjectileLocation`)) 1500.0) false "None")
    (set `self.CanAttack?` false)
    (`KismetSystemLibrary.Delay` 5.0)
    (set `self.CanAttack?` true)))

(fn `Decrease Speed and Height of Jump`
  (params (self2 :type "CharacterMovementComponent Object Reference") (self3 :type "CharacterMovementComponent Object Reference"))
  (set `CharacterMovementComponent.MaxWalkSpeed` 100.0 self2)
  (set `CharacterMovementComponent.JumpZVelocity` 100.0 self3))

(fn `Returning Speed And Jump Values Back`
  (params (self2 :type "CharacterMovementComponent Object Reference") (self3 :type "CharacterMovementComponent Object Reference"))
  (set `CharacterMovementComponent.JumpZVelocity` 420.0 self2)
  (set `CharacterMovementComponent.MaxWalkSpeed` 600.0 self3))

(fn `UserConstructionScript`)